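; BP_CarPawn is a car pawn that handles orbit-camera input and a speed HUD.
; BeginPlay adds the IMC_Movement input context and creates the WB_HUD widget.
; IA_RotateCamera turns the spring arm by sensitivity-scaled input without pitch clamping, and Tick sends scaled CurrentSpeed to the HUD.
; Driving logic and speed calculation are absent from these graphs, and a loop aligning wheel rotations to the collision box is disconnected.
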(event Input|EnhancedActionEvents|EnhancedInputActionIA_RotateCamera
  (params (ActionValue :type Vector%202D%20Structure) (ElapsedSeconds :type Float%20%28double-precision%29) (TriggeredSeconds :type Float%20%28double-precision%29) (InputAction :type Input%20Action%20Object%20Reference :default "/Game/Inputs/InputActions/IA_RotateCamera.IA_RotateCamera"))
  (bind (_x _y) (Math|Vector2D|BreakVector2D ActionValue))
  (bind _camerasensitivity (Variables|Default|GetCameraSensitivity))
  (bind _cameraarm (Variables|Default|GetCameraArm))
  (bind _relativerotation (Variables|/Script/Engine.SceneComponent|GetRelativeRotation _cameraarm))
  (bind (_roll _pitch _yaw) (Math|Rotator|BreakRotator _relativerotation))
  (Transformation|SetRelativeRotation (Variables|Default|GetCameraArm) (Math|Rotator|MakeRotator 0.0 (+ _pitch (* _y _camerasensitivity)) (+ _yaw (* _x _camerasensitivity))) false false))

(event EventBeginPlay
  ;[0.15 0.15 0.15 0.5] Setting up inputs
  (Input|AddMappingContext (PlayerController|LocalPlayerSubsystems|GetEnhancedInputLocalPlayerSubsystem (Game|GetPlayerController 0)) "/Game/Inputs/IMC_Movement.IMC_Movement" 0 "(bIgnoreAllPressedKeysUntilRelease=True,bForceImmediately=False,bNotifyUserSettings=False)")
  ;[0.15 0.15 0.15 0.5] Setting up UI
  (bind _returnvalue (UserInterface|CreateWidget "/Game/UI/WB_HUD.WB_HUD_C"))
  (bind _output_get (Variables|Default|SetHUD _returnvalue))
  (UserInterface|Viewport|AddtoViewport _output_get 0))

(event EventTick
  (params (DeltaSeconds :type Float%20%28single-precision%29))
  ;[0.15 0.15 0.15 0.5] Display speed
  (Default|SetSpeed (Variables|Default|GetHUD) (/ (Variables|Default|GetCurrentSpeed) 10)))

(fn ConstructionScript)