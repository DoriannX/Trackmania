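; Checkpoint actor for a car game that records when a BP_CarPawn drives through it.
; On BeginPlay it adds itself to the total checkpoint count on the BP_GameManager game instance.
; When the car begins overlapping PlayerDetecter, it calls TakeCheckpoint on the pawn and changes the detector's shape color.
; The overlap has no guard, so every re-entry calls TakeCheckpoint again.
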(event OnComponentBeginOverlap(PlayerDetecter)
  (params (OverlappedComponent :type Primitive%20Component%20Object%20Reference) (OtherActor :type Actor%20Object%20Reference) (OtherComp :type Primitive%20Component%20Object%20Reference) (OtherBodyIndex :type Integer) (bFromSweep :type Boolean) (SweepResult :type Hit%20Result%20Structure%20%28by%20ref%29))
  (bind _asbp_car_pawn (Utilities|Casting|CastToBP_CarPawn OtherActor))
  (Default|TakeCheckpoint _asbp_car_pawn)
  (Variables|/Script/Engine.ShapeComponent|SetShapeColor (Variables|Default|GetPlayerDetecter) (Variables|Default|GetColor)))

(event EventBeginPlay
  (bind _asbp_game_manager (Utilities|Casting|CastToBP_GameManager (Game|GetGameInstance)))
  (Variables|/Game/BP_GameManager.BP_GameManager_C|SetTotalCheckpointCount _asbp_game_manager (+ (Variables|/Game/BP_GameManager.BP_GameManager_C|GetTotalCheckpointCount _asbp_game_manager) 1)))

(fn ConstructionScript)